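; Player controller for a modular builder that can pin the mouse cursor in place and swap its icon.
; LockCursor stores the current platform mouse position, sets the locked flag and shows a closed grab hand.
; While locked, Tick snaps the mouse back to that stored, rounded position every frame.
; UnlockCursor clears the flag and sets the open hand cursor.
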(event `self.ReceiveTick`
  (params (DeltaSeconds :type "Float (single-precision)"))
  (bind (_mouse_position_x _mouse_position_y) (`KismetMathLibrary.BreakVector2D` (`self.Mouse Position`)))
  (if (`self.CursorLocked`)
    (`self.SetMouseLocation` (`KismetMathLibrary.Round` _mouse_position_x) (`KismetMathLibrary.Round` _mouse_position_y))))

(event `Lock Cursor`
  (bind _returnvalue (`WidgetLayoutLibrary.GetMousePositionOnPlatform`))
  (set `self.Mouse Position` _returnvalue)
  (set `self.CursorLocked` true)
  (set `self.CurrentMouseCursor` "GrabHandClosed"))

(event `Unlock Cursor`
  (set `self.CursorLocked` false)
  (set `self.CurrentMouseCursor` "Hand"))

(fn `UserConstructionScript`)