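; Free-flying camera pawn for the modular builder, providing navigation and passing building input to the game mode.
; Planar movement input is applied as an unswept actor offset on Tick, while height changes by shifting the movement component's clamped plane constraint and snapping to it.
; Mouse axes yaw the root and pitch the camera; holding Lock Cursor locks the cursor and re-enables controller look input.
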(event `InputAction|Menu`
  (params (Key :type "Key Structure"))
  (:`Pressed`
    (`/Game/Blueprints/ModularBuilderGameMode.Pause` (`self.Game Mode Ref`))))

(event `InputAxis|UpDown`
  (params (AxisValue :type "Float (single-precision)"))
  (bind _movement_component (`self.Movement Component`))
  (bind (_returnvalue_x _returnvalue_y _returnvalue_z) (`KismetMathLibrary.BreakVector` (`MovementComponent.GetPlaneConstraintOrigin` (`self.Movement Component`))))
  (`MovementComponent.SetPlaneConstraintOrigin` _movement_component (`KismetMathLibrary.MakeVector` _returnvalue_x _returnvalue_y (`KismetMathLibrary.FClamp` (+ _returnvalue_z (* AxisValue 50.0)) 200.0 3000.0)))
  (`MovementComponent.SnapUpdatedComponentToPlane` _movement_component))

(event `self.ReceiveBeginPlay`
  (bind _asmodular_builder_game_mode (cast `/Game/Blueprints/ModularBuilderGameMode` (`GameplayStatics.GetGameMode`)))
  (set `self.Game Mode Ref` _asmodular_builder_game_mode)
  (`Controller.SetIgnoreLookInput` (`GameplayStatics.GetPlayerController` 0) true))

(event `InputAction|Snap Roll Left`
  (params (Key :type "Key Structure"))
  (:`Pressed`
    (`/Game/Blueprints/ModularBuilderGameMode.Shape Roll Snap` (`self.Game Mode Ref`) 90.0)))

(event `InputAction|Snap Roll Right`
  (params (Key :type "Key Structure"))
  (:`Pressed`
    (`/Game/Blueprints/ModularBuilderGameMode.Shape Roll Snap` (`self.Game Mode Ref`) -90.0)))

(event `InputAction|Lock Cursor`
  (params (Key :type "Key Structure"))
  (bind _returnvalue (`GameplayStatics.GetPlayerController` 0))
  (:`Pressed`
    (bind _asmodular_builder_controller (cast `/Game/Blueprints/ModularBuilderController` _returnvalue))
    (`/Game/Blueprints/ModularBuilderController.Lock Cursor` _asmodular_builder_controller)
    (`Controller.SetIgnoreLookInput` _returnvalue false))
  (:`Released`
    (bind _asmodular_builder_controller_2 (cast `/Game/Blueprints/ModularBuilderController` _returnvalue))
    (`/Game/Blueprints/ModularBuilderController.Unlock Cursor` _asmodular_builder_controller_2)
    (`Controller.SetIgnoreLookInput` _returnvalue true)))

(event `InputAxis|Shape Roll`
  (params (AxisValue :type "Float (single-precision)"))
  (`/Game/Blueprints/ModularBuilderGameMode.Shape Roll` (`self.Game Mode Ref`) AxisValue))

(event `InputAxis|MouseLeftRight`
  (params (AxisValue :type "Float (single-precision)"))
  (`SceneComponent.K2_AddRelativeRotation` (`self.DefaultSceneRoot`) (`KismetMathLibrary.MakeRotator` 0.0 0.0 AxisValue) false false))

(event `InputAxis|MouseUpDown`
  (params (AxisValue :type "Float (single-precision)"))
  (bind _camera (`self.Camera`))
  (bind (_relativerotation_roll _relativerotation_pitch _relativerotation_yaw) (`KismetMathLibrary.BreakRotator` (`SceneComponent.RelativeRotation` _camera)))
  (`SceneComponent.K2_SetRelativeRotation` _camera (`KismetMathLibrary.MakeRotator` _relativerotation_roll (`KismetMathLibrary.FClamp` (+ AxisValue _relativerotation_pitch) -89.0 89.0) _relativerotation_yaw) false false))

(event `InputAxis|ForwardBackward`
  (params (AxisValue :type "Float (single-precision)"))
  (`self.AddMovementInput` (`SceneComponent.GetForwardVector` (`self.DefaultSceneRoot`)) (* AxisValue 2.0)))

(event `InputAxis|LeftRight`
  (params (AxisValue :type "Float (single-precision)"))
  (`self.AddMovementInput` (`SceneComponent.GetRightVector` (`self.DefaultSceneRoot`)) (* AxisValue 2.0)))

(event `self.ReceiveTick`
  (params (DeltaSeconds :type "Float (single-precision)"))
  (bind _returnvalue (`self.ConsumeMovementInputVector`))
  (`self.K2_AddActorWorldOffset` _returnvalue))

(event `InputAction|Click`
  (params (Key :type "Key Structure"))
  (:`Pressed`
    (`/Game/Blueprints/ModularBuilderGameMode.Click` (`self.Game Mode Ref`))))

(event `InputAction|Mode Switch 1`
  (params (Key :type "Key Structure"))
  (:`Pressed`
    (`/Game/Blueprints/ModularBuilderGameMode.Mode Switch` (`self.Game Mode Ref`) "NewEnumerator0")))

(event `InputAction|Mode Switch 2`
  (params (Key :type "Key Structure"))
  (:`Pressed`
    (`/Game/Blueprints/ModularBuilderGameMode.Mode Switch` (`self.Game Mode Ref`) "NewEnumerator1")))

(event `InputAction|Mode Switch 3`
  (params (Key :type "Key Structure"))
  (:`Pressed`
    (`/Game/Blueprints/ModularBuilderGameMode.Mode Switch` (`self.Game Mode Ref`) "NewEnumerator2")))

(event `InputAction|Mode Switch 4`
  (params (Key :type "Key Structure"))
  (:`Pressed`
    (`/Game/Blueprints/ModularBuilderGameMode.Mode Switch` (`self.Game Mode Ref`) "NewEnumerator4")))

(event `InputAction|Snap`
  (params (Key :type "Key Structure"))
  (:`Pressed`
    (`/Game/Blueprints/ModularBuilderGameMode.Grid Snap` (`self.Game Mode Ref`))))

(fn `UserConstructionScript`)