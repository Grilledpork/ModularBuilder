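; Game mode for a modular builder where the player places, moves, deletes and re-materials cubes, cylinders and wedges, with HUD and pause menu.
; A mode state machine routes clicks and key switches, all targeting through a mouse-cursor line trace.
; Tick aligns a ghost preview to the hit surface normal, with optional grid snapping and adjustable roll.
; Moving destroys the picked object and enters Replace mode until it is placed again.
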(event `self.ReceiveBeginPlay`
  (bind _returnvalue (`|CreateWidget` "/Game/UI/WBP_HUD.WBP_HUD_C" (`GameplayStatics.GetPlayerController` 0)))
  (bind _output_get (set `self.HUD Ref` _returnvalue))
  (`UserWidget.AddToViewport` _output_get 0)
  (`self.Enter Placement Mode`))

(event `Grid Snap`
  (bind _isa (`/Engine/EditorBlueprintResources/StandardMacros.FlipFlop`)
    (:`A`
      _)
    (:`B`
      _))
  (bind _output_get (set `self.Grid Snap Enabled` _isa))
  (`/Game/UI/WBP_HUD.Toggle Snap` (`self.HUD Ref`) _output_get))

(event `Select Object`
  (bind (_hit _return_value) (`self.Pointer Trace`))
  (if _return_value
    (switch `/Game/Blueprints/Modes` (`self.Current Mode`)
      (:`NewEnumerator1`
        (bind _output_get (set `self.Selected Object` (`.HitActor` (`GameplayStatics.BreakHitResult` _hit))))
        (cast `/Game/Blueprints/Objects/PlacableObjectCube` _output_get
          (:`then`
            (set `self.Current Shape ID` 0))
          (:`CastFailed`
            (cast `/Game/Blueprints/Objects/PlacableObjectCylinder` _output_get
              (:`then`
                (set `self.Current Shape ID` 1))
              (:`CastFailed`
                (cast `/Game/Blueprints/Objects/PlacableObjectWedge` _output_get)
                (set `self.Current Shape ID` 2)))))
        (`self.Enter Replace Mode`)
        (`self.K2_DestroyActor` (`self.Selected Object`)))
      (:`NewEnumerator2`
        (if (`self.ActorHasTag` (`.HitActor` (`GameplayStatics.BreakHitResult` _hit)) "Selectable")
          (`self.K2_DestroyActor` (`.HitActor` (`GameplayStatics.BreakHitResult` _hit)))))
      (:`NewEnumerator4`
        (set `self.Selected Object` (`.HitActor` (`GameplayStatics.BreakHitResult` _hit)))
        (`self.Material Swap`)))))

(event `Place Object Snap`
  (bind (_hit _return_value) (`self.Pointer Trace`))
  (if _return_value
    (bind (_returnvalue_roll _returnvalue_pitch _returnvalue_yaw) (`KismetMathLibrary.BreakRotator` (`KismetMathLibrary.Conv_VectorToRotator` (`.Normal` (`GameplayStatics.BreakHitResult` _hit)))))
    (`|SpawnActorFromClass` (`|GetArrayItem` (`self.Meshes`) (`self.Current Shape ID`)) (`KismetMathLibrary.MakeTransform` (`KismetMathLibrary.MakeVector` (`self.Round To` (.x (+ (`.Location` (`GameplayStatics.BreakHitResult` _hit)) (* (`.Normal` (`GameplayStatics.BreakHitResult` _hit)) 50.0))) 100.0) (`self.Round To` (.y (+ (`.Location` (`GameplayStatics.BreakHitResult` _hit)) (* (`.Normal` (`GameplayStatics.BreakHitResult` _hit)) 50.0))) 100.0) (`self.Round To` (.z (+ (`.Location` (`GameplayStatics.BreakHitResult` _hit)) (* (`.Normal` (`GameplayStatics.BreakHitResult` _hit)) 50.0))) 100.0)) (`KismetMathLibrary.MakeRotator` (`self.Snap Roll Value`) (`self.Round To` _returnvalue_pitch 90.0) (`self.Round To` _returnvalue_yaw 90.0))) "AdjustIfPossibleButDontSpawnIfColliding" "OverrideRootScale" null null)
    (if (`|EnumEquality` (`self.Current Mode`) "NewEnumerator3")
      (`self.Exit Placement Mode`)
      (bind _output_get (set `self.Current Mode` "NewEnumerator1"))
      (`/Game/UI/WBP_HUD.Change Active Mode` (`self.HUD Ref`) _output_get))))

(event `Place Object`
  (bind (_hit _return_value) (`self.Pointer Trace`))
  (if _return_value
    (bind _returnvalue (`|SpawnActorFromClass` (`|GetArrayItem` (`self.Meshes`) (`self.Current Shape ID`)) (`KismetMathLibrary.MakeTransform` (+ (`.Location` (`GameplayStatics.BreakHitResult` _hit)) (* (`.Normal` (`GameplayStatics.BreakHitResult` _hit)) 51.0)) (`KismetMathLibrary.Conv_VectorToRotator` (`.Normal` (`GameplayStatics.BreakHitResult` _hit)))) "AdjustIfPossibleButDontSpawnIfColliding" "OverrideRootScale" null null))
    (`/Engine/EditorBlueprintResources/StandardMacros.IsValid` _returnvalue
      (:`Is Valid`
        (`self.K2_AddActorLocalRotation` _returnvalue (`KismetMathLibrary.MakeRotator` (`self.Roll Value`) 0.0) false false)
        (if (`|EnumEquality` (`self.Current Mode`) "NewEnumerator3")
          (`self.Exit Placement Mode`)
          (bind _output_get (set `self.Current Mode` "NewEnumerator1"))
          (`/Game/UI/WBP_HUD.Change Active Mode` (`self.HUD Ref`) _output_get))))))

(event `Shape Roll`
  (params (`Axis Value` :type "Float (double-precision)"))
  (bind _current_mode (`self.Current Mode`))
  (bind _ghost_object (`self.Ghost Object`))
  (if (or (`|EnumEquality` _current_mode "NewEnumerator0") (`|EnumEquality` _current_mode "NewEnumerator3"))
    (if (`self.Grid Snap Enabled`)
      (`self.K2_AddActorLocalRotation` _ghost_object (`KismetMathLibrary.MakeRotator` (`self.Snap Roll Value`)) false false)
      (else
        (bind _output_get (set `self.Roll Value` (+ (`self.Roll Value`) `Axis Value`)))
        (`self.K2_AddActorLocalRotation` _ghost_object (`KismetMathLibrary.MakeRotator` _output_get) false false)))))

(event `self.ReceiveTick`
  (params (DeltaSeconds :type "Float (single-precision)"))
  (if (`self.Grid Snap Enabled`)
    (`self.Set Ghost Snap`)
    (else
      (`self.Set Ghost`))))

(event `Set Ghost`
  (bind _ghost_object (`self.Ghost Object`))
  (bind _current_mode (`self.Current Mode`))
  (if (or (`|EnumEquality` _current_mode "NewEnumerator0") (`|EnumEquality` _current_mode "NewEnumerator3"))
    (bind (_hit _return_value) (`self.Pointer Trace`))
    (if _return_value
      (`self.K2_SetActorLocationAndRotation` _ghost_object (+ (`.Location` (`GameplayStatics.BreakHitResult` _hit)) (* (`.Normal` (`GameplayStatics.BreakHitResult` _hit)) 51.0)) (`KismetMathLibrary.Conv_VectorToRotator` (`.Normal` (`GameplayStatics.BreakHitResult` _hit))) false false)
      (`self.SetActorHiddenInGame` _ghost_object false)
      (else
        (`self.SetActorHiddenInGame` _ghost_object true)))))

(event `Shape Roll Snap`
  (params (`Snap Value` :type "Float (double-precision)"))
  (bind _current_mode (`self.Current Mode`))
  (if (and (or (`|EnumEquality` _current_mode "NewEnumerator0") (`|EnumEquality` _current_mode "NewEnumerator3")) (`self.Grid Snap Enabled`))
    (set `self.Snap Roll Value` (+ (`self.Snap Roll Value`) `Snap Value`))))

(event `Set Ghost Snap`
  (bind _current_mode (`self.Current Mode`))
  (if (or (`|EnumEquality` _current_mode "NewEnumerator0") (`|EnumEquality` _current_mode "NewEnumerator3"))
    (bind (_hit _return_value) (`self.Pointer Trace`))
    (if _return_value
      (`self.K2_SetActorLocationAndRotation` (`self.Ghost Object`) (`KismetMathLibrary.MakeVector` (`self.Round To` (.x (+ (`.Location` (`GameplayStatics.BreakHitResult` _hit)) (* (`.Normal` (`GameplayStatics.BreakHitResult` _hit)) 50.0))) 100.0) (`self.Round To` (.y (+ (`.Location` (`GameplayStatics.BreakHitResult` _hit)) (* (`.Normal` (`GameplayStatics.BreakHitResult` _hit)) 50.0))) 100.0) (`self.Round To` (.z (+ (`.Location` (`GameplayStatics.BreakHitResult` _hit)) (* (`.Normal` (`GameplayStatics.BreakHitResult` _hit)) 50.0))) 100.0)) (`KismetMathLibrary.Conv_VectorToRotator` (`.Normal` (`GameplayStatics.BreakHitResult` _hit))) false false))))

(event `Click`
  (switch `/Game/Blueprints/Modes` (`self.Current Mode`)
    (:`NewEnumerator0`
      (if (`self.Grid Snap Enabled`) :!label _label
        (`self.Place Object Snap`)
        (else
          (`self.Place Object`))))
    (:`NewEnumerator1`
      (`self.Select Object` :!label _label_2))
    (:`NewEnumerator3`
      (goto _label))
    (:`NewEnumerator2`
      (goto _label_2))
    (:`NewEnumerator4`
      (goto _label_2))))

(event `Mode Switch`
  (params (`Mode Key` :type "/Game/Blueprints/Modes Enum" :default "NewEnumerator0"))
  (if (not (`|EnumEquality` (`self.Current Mode`) "NewEnumerator3"))
    (switch `/Game/Blueprints/Modes` `Mode Key`
      (:`NewEnumerator0`
        (if (`|EnumEquality` (`self.Current Mode`) "NewEnumerator0")
          (`self.Shape Swap`)
          (else
            (`self.Enter Placement Mode`))))
      (:`NewEnumerator1`
        (if (`|EnumEquality` (`self.Current Mode`) "NewEnumerator0")
          (`self.Exit Placement Mode`))
        (bind _output_get (set `self.Current Mode` "NewEnumerator1"))
        (`/Game/UI/WBP_HUD.Change Active Mode` (`self.HUD Ref`) _output_get))
      (:`NewEnumerator2`
        (if (`|EnumEquality` (`self.Current Mode`) "NewEnumerator0")
          (`self.Exit Placement Mode`))
        (bind _output_get_2 (set `self.Current Mode` "NewEnumerator2"))
        (`/Game/UI/WBP_HUD.Change Active Mode` (`self.HUD Ref`) _output_get_2))
      (:`NewEnumerator4`
        (if (`|EnumEquality` (`self.Current Mode`) "NewEnumerator0")
          (`self.Exit Placement Mode`))
        (bind _output_get_3 (set `self.Current Mode` "NewEnumerator4"))
        (`/Game/UI/WBP_HUD.Change Active Mode` (`self.HUD Ref`) _output_get_3)))))

(event `Enter Placement Mode`
  (bind _output_get (set `self.Current Mode` "NewEnumerator0"))
  (`/Game/UI/WBP_HUD.Change Active Mode` (`self.HUD Ref`) _output_get)
  (bind _returnvalue (`|SpawnActorFromClass` (`|GetArrayItem` (`self.GhostMeshes`) (`self.Current Shape ID`)) (`KismetMathLibrary.MakeTransform` (0.0 0.0 0.0)) "AdjustIfPossibleButAlwaysSpawn" "OverrideRootScale" null null :!label _label_3))
  (set `self.Ghost Object` _returnvalue))

(event `Enter Replace Mode`
  (bind _output_get (set `self.Current Mode` "NewEnumerator3"))
  (`/Game/UI/WBP_HUD.Change Active Mode` (`self.HUD Ref`) _output_get)
  (goto _label_3))

(event `Shape Swap`
  (bind _result (`/Engine/EditorBlueprintResources/StandardMacros.IncrementInt` (`self.Current Shape ID`))
    (:`  `
      (set `self.Current Shape ID` (mod _result 3))
      (`self.K2_DestroyActor` (`self.Ghost Object`))
      (goto _label_3))))

(event `Exit Placement Mode`
  (`self.K2_DestroyActor` (`self.Ghost Object`)))

(event `Pause`
  (bind _returnvalue (`|CreateWidget` "/Game/UI/WBP_Menu.WBP_Menu_C"))
  (`UserWidget.AddToViewport` _returnvalue 0)
  (`Widget.SetVisibility` (`self.HUD Ref`) "HitTestInvisible")
  (`GameplayStatics.SetGamePaused` true))

(event `Exit Pause`
  (params (`Pause Menu` :type "/Game/UI/WBP_Menu Object Reference"))
  (`Widget.RemoveFromParent` `Pause Menu`)
  (`Widget.SetVisibility` (`self.HUD Ref`) "Visible")
  (`GameplayStatics.SetGamePaused` false))

(event `Material Swap`
  (bind _selected_object (`self.Selected Object`))
  (bind _asplacable_object_cube (cast `/Game/Blueprints/Objects/PlacableObjectCube` _selected_object)
    (:`then`
      (bind _result (`/Engine/EditorBlueprintResources/StandardMacros.IncrementInt` (`/Game/Blueprints/Objects/PlacableObjectParent.Material ID` _asplacable_object_cube))
        (:`  `
          (bind _output_get (set `/Game/Blueprints/Objects/PlacableObjectParent.Material ID` (mod _result 8) _asplacable_object_cube))
          (`PrimitiveComponent.SetMaterial` (`/Game/Blueprints/Objects/PlacableObjectParent.Shape` _asplacable_object_cube) 0 (`|GetArrayItem` (`self.Materials`) _output_get)))))
    (:`CastFailed`
      (bind _asplacable_object_cylinder (cast `/Game/Blueprints/Objects/PlacableObjectCylinder` _selected_object)
        (:`then`
          (bind _result_2 (`/Engine/EditorBlueprintResources/StandardMacros.IncrementInt` (`/Game/Blueprints/Objects/PlacableObjectParent.Material ID` _asplacable_object_cylinder))
            (:`  `
              (bind _output_get_2 (set `/Game/Blueprints/Objects/PlacableObjectParent.Material ID` (mod _result_2 8) _asplacable_object_cylinder))
              (`PrimitiveComponent.SetMaterial` (`/Game/Blueprints/Objects/PlacableObjectParent.Shape` _asplacable_object_cylinder) 0 (`|GetArrayItem` (`self.Materials`) _output_get_2)))))
        (:`CastFailed`
          (bind _asplacable_object_wedge (cast `/Game/Blueprints/Objects/PlacableObjectWedge` _selected_object))
          (bind _result_3 (`/Engine/EditorBlueprintResources/StandardMacros.IncrementInt` (`/Game/Blueprints/Objects/PlacableObjectParent.Material ID` _asplacable_object_wedge))
            (:`  `
              (bind _output_get_3 (set `/Game/Blueprints/Objects/PlacableObjectParent.Material ID` (mod _result_3 8) _asplacable_object_wedge))
              (`PrimitiveComponent.SetMaterial` (`/Game/Blueprints/Objects/PlacableObjectParent.Shape` _asplacable_object_wedge) 0 (`|GetArrayItem` (`self.Materials`) _output_get_3)))))))))

(fn `Pointer Trace`
  (returns (Hit :type "HitResult Structure") (`Return Value` :type Boolean))
  (bind (_worldlocation _worlddirection _returnvalue) (`PlayerController.DeprojectMousePositionToWorld` (`GameplayStatics.GetPlayerController` 0)))
  (if _returnvalue
    (bind (_outhit _returnvalue_2) (`KismetSystemLibrary.LineTraceSingle` :`Start` _worldlocation :`End` (+ _worldlocation (* _worlddirection 10000.0)) :`TraceChannel` "TraceTypeQuery3" :`DrawDebugType` "ForOneFrame"))
    (return _outhit _returnvalue_2)
    (else
      (return (struct) false))))

(fn `UserConstructionScript`)